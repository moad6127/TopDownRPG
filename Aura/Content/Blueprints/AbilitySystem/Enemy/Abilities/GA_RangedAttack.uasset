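; Enemy ranged attack gameplay ability that fires a projectile at the avatar's combat target.
; On activation it turns the avatar toward the target, caches the target's location and plays a random tagged attack montage from the avatar.
; A one-shot wait for the montage's gameplay event tag triggers SpawnProjectile from that montage's socket tag with an overridden pitch.
; The graph never calls EndAbility.
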(event `self.K2_ActivateAbility`
  (bind _returnvalue (`self.GetAvatarActorFromActorInfo`))
  (bind (_taggedmontage_montage _taggedmontage_montagetag _taggedmontage_sockettag) (break `TaggedMontage` (`self.TaggedMontage`)))
  (bind _returnvalue_2 (message `EnemyInterface.GetCombatTarget` _returnvalue))
  (bind _returnvalue_3 (`Actor.K2_GetActorLocation` _returnvalue_2))
  (message `CombatInterface.UpdateFacingTarget` _returnvalue _returnvalue_3)
  (set `self.Projectile Target Location` _returnvalue_3)
  (bind _returnvalue_4 (message `CombatInterface.GetAttackMontages` (`self.GetAvatarActorFromActorInfo`)))
  (bind _output_get (set `self.TaggedMontage` (`self.GetRandomTaggedMontageFromArray` _returnvalue_4)))
  (bind (_montage _montagetag) (break `TaggedMontage` _output_get))
  (`AbilityTask_PlayMontageAndWait.CreatePlayMontageAndWaitProxy` "None" _montage 1.0 "None" false
    (:`then`
      (`AbilityTask_WaitGameplayEvent.WaitGameplayEvent` _montagetag null true
        (:`EventReceived`
          (`self.SpawnProjectile` (`self.Projectile Target Location`) _taggedmontage_sockettag true 20.0))))))